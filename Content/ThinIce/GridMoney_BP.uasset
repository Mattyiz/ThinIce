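; GridMoney_BP is the money tile in the Thin Ice grid, identified as type 6.
; On BeginPlay it caches the player and game manager, and applies the money material to its cube only if the game instance's previous ice remaining is zero or less.
; It then waits a delay scaled by its X and Y position so tiles register in order, adding itself to the manager's YGrid row derived from 250-unit spacing.
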(event Collision|EventActorBeginOverlap
  (params (OtherActor :type Actor%20Object%20Reference))
  (|CallParentFunction OtherActor) ; This node is disabled and will not be called.\nDrag off pins to build functionality.
)

(event EventTick
  (params (DeltaSeconds :type Float%20%28single-precision%29))
  (|CallParentFunction DeltaSeconds) ; This node is disabled and will not be called.\nDrag off pins to build functionality.
)

(event EventBeginPlay
  (bind _cube (Variables|Default|GetCube))
  (bind _returnvalue (Transformation|GetWorldTransform _cube))
  (bind _returnvalue_2 (/ (.y (.location _returnvalue)) 2.5e+02))
  (bind _returnvalue_3 (Math|Float|Truncate _returnvalue_2))
  (Variables|Default|SetType 6)
  (bind _outactors (Actor|GetAllActorsOfClass "/Game/ThinIce/Player_BP.Player_BP_C"))
  (Variables|Default|SetPlayer (Utilities|Array|Get(acopy) _outactors))
  (bind _outactors_2 (Actor|GetAllActorsOfClass "/Game/ThinIce/GameManager_BP.GameManager_BP_C"))
  (bind _output_get (Variables|Default|SetManager (Utilities|Array|Get(acopy) _outactors_2)))
  (bind _asice_counter_instance (Utilities|Casting|CastToIceCounterInstance (Game|GetGameInstance)))
  (if (<= (Variables|/Game/ThinIce/IceCounterInstance.IceCounterInstance_C|GetPreviousIceRemaining _asice_counter_instance) 0)
    (Rendering|Material|SetMaterial (Variables|Default|GetCube) 0 "/Game/ThinIce/Materials/Money_Mat.Money_Mat"))
  (Utilities|FlowControl|Delay (+ (/ _returnvalue_2 4.7) (/ (/ (.x (.location _returnvalue)) 2.5e+02) 4.7))) ; Delays based on the cordinates of the object. This will ensure they get added in the right order
  (if (>= (Utilities|Array|Length (Variables|/Game/ThinIce/GameManager_BP.GameManager_BP_C|GetYGrid _output_get)) (+ _returnvalue_3 1)) ; If there is a spot in the ygrid  continue, if not add a spot then continue
    _
    (else
      (Utilities|Array|Add :TargetArray (Variables|/Game/ThinIce/GameManager_BP.GameManager_BP_C|GetYGrid _output_get))))
  (Utilities|Array|Add (Utilities|Struct|BreakXGrid (Utilities|Array|Get(acopy) (Variables|/Game/ThinIce/GameManager_BP.GameManager_BP_C|GetYGrid _output_get) _returnvalue_3)) self))

(fn ConstructionScript
  (|CallParentFunction))