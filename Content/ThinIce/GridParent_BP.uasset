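; GridParent_BP is a grid square actor for ThinIce, apparently a base for tile types, that registers itself with the game manager at startup.
; On BeginPlay it finds GameManager_BP and converts its Cube's world position into grid indices using a fixed cell size.
; A position-based Delay staggers registration so squares append in order to the manager's nested YGrid array, adding a row when missing.
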(event EventBeginPlay
  (bind _cube (Variables|Default|GetCube))
  (bind _returnvalue (Transformation|GetWorldTransform _cube))
  (bind _returnvalue_2 (/ (.y (.location _returnvalue)) 2.5e+02))
  (bind _returnvalue_3 (Math|Float|Truncate _returnvalue_2))
  (bind _outactors (Actor|GetAllActorsOfClass "/Game/ThinIce/GameManager_BP.GameManager_BP_C"))
  (bind _output_get (Variables|Default|SetManager (Utilities|Array|Get(acopy) _outactors)))
  (Utilities|FlowControl|Delay (+ (/ _returnvalue_2 5.0) (/ (/ (.x (.location _returnvalue)) 2.5e+02) 5.0))) ; Delays based on the cordinates of the object. This will ensure they get added in the right order
  (if (>= (Utilities|Array|Length (Variables|/Game/ThinIce/GameManager_BP.GameManager_BP_C|GetYGrid _output_get)) (+ _returnvalue_3 1)) ; If there is a spot in the ygrid  continue, if not add a spot then continue
    _
    (else
      (Utilities|Array|Add :TargetArray (Variables|/Game/ThinIce/GameManager_BP.GameManager_BP_C|GetYGrid _output_get))))
  (Utilities|Array|Add (Utilities|Struct|BreakXGrid (Utilities|Array|Get(acopy) (Variables|/Game/ThinIce/GameManager_BP.GameManager_BP_C|GetYGrid _output_get) _returnvalue_3)) self))

(event Collision|EventActorBeginOverlap
  (params (OtherActor :type Actor%20Object%20Reference)))

(event EventTick
  (params (DeltaSeconds :type Float%20%28single-precision%29)))

(fn ConstructionScript)