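; Player Blueprint for ThinIce that moves a sphere in discrete steps along world X and Y.
; Up, Down, Left and Right presses each offset the Sphere by MoveAmount, then print its position scaled to what appear to be grid coordinates.
; BeginPlay caches the first GameManager_BP as Manager, which is not yet used.
; CanMove is an uncalled stub returning false, so movement is unchecked.
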(event EventBeginPlay
  (bind _outactors (Actor|GetAllActorsOfClass "/Game/ThinIce/GameManager_BP.GameManager_BP_C"))
  (Variables|Default|SetManager (Utilities|Array|Get(acopy) _outactors)))

(event Collision|EventActorBeginOverlap
  (params (OtherActor :type Actor%20Object%20Reference)))

(event EventTick
  (params (DeltaSeconds :type Float%20%28single-precision%29)))

(event Input|ActionEvents|InputActionLeft
  (params (Key :type Key%20Structure :default "None"))
  (bind _sphere (Variables|Default|GetSphere))
  (bind _returnvalue (Transformation|GetWorldLocation _sphere))
  (:Pressed
    (Transformation|AddWorldOffset (Variables|Default|GetSphere) (Math|Vector|MakeVector 0.0 (* (Variables|Default|GetMoveAmount) -1.0) 0.0) false false)
    (Development|PrintString (Utilities|String|Append (Utilities|String|Append "Y: " (Utilities|String|ToString(Float) (/ (.y _returnvalue) 2.5e+02))) (Utilities|String|Append " X: " (Utilities|String|ToString(Float) (/ (.x _returnvalue) 2.5e+02)))))))

(event Input|ActionEvents|InputActionRight
  (params (Key :type Key%20Structure :default "None"))
  (bind _sphere (Variables|Default|GetSphere))
  (bind _returnvalue (Transformation|GetWorldLocation _sphere))
  (:Pressed
    (Transformation|AddWorldOffset (Variables|Default|GetSphere) (Math|Vector|MakeVector 0.0 (Variables|Default|GetMoveAmount) 0.0) false false)
    (Development|PrintString (Utilities|String|Append (Utilities|String|Append "Y: " (Utilities|String|ToString(Float) (/ (.y _returnvalue) 2.5e+02))) (Utilities|String|Append " X: " (Utilities|String|ToString(Float) (/ (.x _returnvalue) 2.5e+02)))))))

(event Input|ActionEvents|InputActionDown
  (params (Key :type Key%20Structure :default "None"))
  (bind _sphere (Variables|Default|GetSphere))
  (bind _returnvalue (Transformation|GetWorldLocation _sphere))
  (:Pressed
    (Transformation|AddWorldOffset (Variables|Default|GetSphere) (Math|Vector|MakeVector (* (Variables|Default|GetMoveAmount) -1.0) 0.0 0.0) false false)
    (Development|PrintString (Utilities|String|Append (Utilities|String|Append "Y: " (Utilities|String|ToString(Float) (/ (.y _returnvalue) 2.5e+02))) (Utilities|String|Append " X: " (Utilities|String|ToString(Float) (/ (.x _returnvalue) 2.5e+02)))))))

(event Input|ActionEvents|InputActionUp
  (params (Key :type Key%20Structure :default "None"))
  (bind _sphere (Variables|Default|GetSphere))
  (bind _returnvalue (Transformation|GetWorldLocation _sphere))
  (:Pressed
    (Transformation|AddWorldOffset (Variables|Default|GetSphere) (Math|Vector|MakeVector (Variables|Default|GetMoveAmount) 0.0 0.0) false false)
    (Development|PrintString (Utilities|String|Append (Utilities|String|Append "Y: " (Utilities|String|ToString(Float) (/ (.y _returnvalue) 2.5e+02))) (Utilities|String|Append " X: " (Utilities|String|ToString(Float) (/ (.x _returnvalue) 2.5e+02)))))))

(fn ConstructionScript)

(fn CanMove
  (params (X :type Float%20%28double-precision%29) (Y :type Float%20%28double-precision%29))
  (return false))